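; Lightning orb VFX actor that loops a burst of particle lights spreading outward around a center particle.
; After a short startup delay, BeginPlay spawns NumLights particle components from a template and starts a repeating reset timer.
; Tick uses curves to drive their evenly spaced ring's radius and rotation, plus each light's XY scale.
; Each reset pauses motion, restarts the center particle, then briefly afterward recenters and reactivates the lights.
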(event `self.ReceiveTick`
  (params (DeltaSeconds :type "Float (single-precision)"))
  (bind _returnvalue (`CurveFloat.GetFloatValue` (`self.ScaleCurve`) (`self.Time`)))
  (set `self.Delta` DeltaSeconds)
  (if (`self.bEnabled`)
    (bind _output_get (set `self.Time` (+ DeltaSeconds (`self.Time`))))
    (bind _output_get_2 (set `self.Alpha` (`CurveFloat.GetFloatValue` (`self.Curve`) (`KismetMathLibrary.NormalizeToRange` _output_get 0.0 (`self.Overtime`)))))
    (`KismetSystemLibrary.PrintString` (`KismetStringLibrary.Conv_DoubleToString` _output_get_2) false false)
    (for (_array_element _array_index) (`self.FxList`)
      (`SceneComponent.K2_SetRelativeLocation` _array_element (* (`KismetMathLibrary.GetForwardVector` (`KismetMathLibrary.MakeRotator` 0.0 0.0 (+ (* _array_index (`KismetMathLibrary.Conv_IntToDouble` (/ 360 (`self.NumLights`)))) (`KismetMathLibrary.Lerp` 0.0 (`self.AddedRotationAtEnd`) (`self.Alpha`))))) (`KismetMathLibrary.Lerp` 0.0 (`self.MaxCricleSize`) (`KismetMathLibrary.FClamp` (`self.Alpha`)))) false false)
      (`SceneComponent.SetRelativeScale3D` _array_element (`KismetMathLibrary.MakeVector` _returnvalue _returnvalue 1.0)))))

(event `self.ReceiveBeginPlay`
  (`KismetSystemLibrary.Delay` 1.0)
  (for _ (range (`self.NumLights`))
    (bind _returnvalue (`AddComponent|NODE_AddParticleSystemComponent-0`))
    (`ParticleSystemComponent.SetTemplate` _returnvalue (`self.Template`))
    (`KismetArrayLibrary.Array_Add` (`self.FxList`) _returnvalue))
  (set `self.bEnabled` true)
  (`ActorComponent.Activate` (`self.CenterParticle`) true)
  (`KismetSystemLibrary.K2_SetTimerDelegate` (delegate `Reset`) 2.0 true))

(event `Reset`
  (set `self.bEnabled` false)
  (`ActorComponent.SetActive` (`self.CenterParticle`) true true)
  (`KismetSystemLibrary.K2_SetTimerDelegate` (delegate `Timed`) 0.2))

(event `Timed`
  (for _array_element (`self.FxList`)
    (`ActorComponent.Deactivate` _array_element)
    (`SceneComponent.K2_SetRelativeLocation` _array_element (0.0 0.0 0.0) false false)
    (`ActorComponent.Activate` _array_element true))
  (set `self.Time` 0.0)
  (set `self.bEnabled` true))

(fn `UserConstructionScript`)