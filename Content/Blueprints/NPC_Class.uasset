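; Base NPC character that can move around, react to the player and trigger a cinematic.
; A self-repeating, delayed move event sends it through its AI controller either to random navigable points around its spawn location or cyclically along an array of target points.
; An interaction box flags it as highlighted while the player overlaps, optionally launching them upward.
; PlayCinematic creates a level sequence player and passes it to KeyOfLifeGameMode.
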(event `self.ReceiveBeginPlay`
  ;[1 1 1] BeginPlay
  (`|ExecutionSequence`
    (:`then_0`
      (set `CharacterMovementComponent.MaxWalkSpeed` (`self.MoveSpeed`) (`self.CharacterMovement`)))
    (:`then_1`
      (`self.SetSpawnLocationAsDefaultLocation`))
    (:`then_2`
      ;;[1 1 1] Wanders if it is flagged to
      (if (`self.Moves`)
        (`self.MoveEvent`)))))

(event `self.InteractionBox.OnComponentBeginOverlap`
  (params (OverlappedComponent :type "PrimitiveComponent Object Reference") (OtherActor :type "Actor Object Reference") (OtherComp :type "PrimitiveComponent Object Reference") (OtherBodyIndex :type Integer) (bFromSweep :type Boolean) (SweepResult :type "HitResult Structure (by ref)"))
  ;[1 1 1] NPC is interactable by the Player if he is within range
  (if (== OtherActor (`GameplayStatics.GetPlayerCharacter` 0))
    (if (`self.InteractsWithPlayer`)
      (set `self.Highlighted` true)
      (if (`self.LaunchesPlayer`)
        (`self.LaunchMainCharacter`)))))

(event `self.InteractionBox.OnComponentEndOverlap`
  (params (OverlappedComponent :type "PrimitiveComponent Object Reference") (OtherActor :type "Actor Object Reference") (OtherComp :type "PrimitiveComponent Object Reference") (OtherBodyIndex :type Integer))
  ;[1 1 1] NPC is interactable by the Player if he is within range
  (if (== OtherActor (`GameplayStatics.GetPlayerCharacter` 0))
    (if (`self.InteractsWithPlayer`)
      (set `self.Highlighted` false))))

(event `MoveEvent`
  ;[1 1 1] Moving: Wander or Patrolling
  (if (`self.RandomWander`)
    (`AIController.MoveToLocation` (`AIBlueprintHelperLibrary.GetAIController` self) (`NavigationSystemV1.K2_GetRandomLocationInNavigableRadius` (`self.DefaultLocation`) (`self.WanderRange`) null null) -1.0 true true true true null true)
    (else
      (`/Engine/EditorBlueprintResources/StandardMacros.IsValid` (`|GetArrayItem` (`self.TargetPointsArray`) (`self.Choice`))
        (:`Is Valid`
          (`AIController.MoveToLocation` (`AIBlueprintHelperLibrary.GetAIController` self) (`self.K2_GetActorLocation` (`|GetArrayItem` (`self.TargetPointsArray`) (`self.Choice`))) -1.0 true true true true null true)
          (`/Engine/EditorBlueprintResources/StandardMacros.IncrementInt` (`self.Choice`)
            (:`  `
              (`/Engine/EditorBlueprintResources/StandardMacros.IsValid` (`|GetArrayItem` (`self.TargetPointsArray`) (`self.Choice`))
                (:`Is Valid`
                  _)
                (:`Is Not Valid`
                  (set `self.Choice` 0)))))))))
  (`KismetSystemLibrary.Delay` (`self.MoveDelay`))
  (`self.MoveEvent`))

(event `SetSpawnLocationAsDefaultLocation`
  ;[1 1 1] Set Default Location
  (set `self.DefaultLocation` (`self.K2_GetActorLocation` (`Controller.K2_GetPawn` (`self.GetController`)))))

(event `PlayCinematic`
  ;[1 1 1] PlayCinematic
  (`/Engine/EditorBlueprintResources/StandardMacros.IsValid` (`self.LevelSequence`)
    (:`Is Valid`
      (bind (_outactor _returnvalue) (`LevelSequencePlayer.CreateLevelSequencePlayer` (`self.LevelSequence`)))
      (bind _outactors (`GameplayStatics.GetAllActorsOfClass` "/Game/Blueprints/KeyOfLifeGameMode.KeyOfLifeGameMode_C"))
      (for _array_element _outactors
        (`/Game/Blueprints/KeyOfLifeGameMode.PlayLevelSequence` _array_element _returnvalue)))))

(event `LaunchMainCharacter`
  (`self.LaunchCharacter` (`GameplayStatics.GetPlayerCharacter` 0) (0.0 0.0 1000.0) false false))

(fn `UserConstructionScript`)