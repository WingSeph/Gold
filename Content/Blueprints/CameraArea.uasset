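; CameraArea is a trigger volume that switches the player's view to its own camera when the player character overlaps its box.
; If overlap-activated, entering briefly disables input, blends the view, aligns control rotation and flags the change on MainCharacter; leaving blends back.
; A single-timed option holds the shot for a set time, returns to the player and destroys the actor.
; Entry can also animate text on a UI_TextBox widget.
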(event `self.Box.OnComponentBeginOverlap`
  (params (OverlappedComponent :type "PrimitiveComponent Object Reference") (OtherActor :type "Actor Object Reference") (OtherComp :type "PrimitiveComponent Object Reference") (OtherBodyIndex :type Integer) (bFromSweep :type Boolean) (SweepResult :type "HitResult Structure (by ref)"))
  ;[1 1 1] Overlapping Event
  (if (== OtherActor (`GameplayStatics.GetPlayerCharacter` 0))
    (if (`self.DisplayWidget`)
      (`self.AnimateWidgetText`))
    (if (`self.ActivatedWithOverlap`)
      (`self.DisablePlayerInput`)
      (`self.BlendToCamera`)
      (if (`self.SingleTimedInstance`)
        (`self.SingleTimedInstanceEvent`)))))

(event `self.Box.OnComponentEndOverlap`
  (params (OverlappedComponent :type "PrimitiveComponent Object Reference") (OtherActor :type "Actor Object Reference") (OtherComp :type "PrimitiveComponent Object Reference") (OtherBodyIndex :type Integer))
  ;[1 1 1] Overlapping Event
  (if (== OtherActor (`GameplayStatics.GetPlayerCharacter` 0))
    (if (`self.IsOverlappingActor` (`GameplayStatics.GetPlayerCharacter` 0))
      _
      (elif (`self.ActivatedWithOverlap`)
        (`self.BlendToPlayerCamera`)))))

(event `BlendToCamera`
  ;[1 1 1] Blend to this camera
  (`PlayerController.SetViewTargetWithBlend` (`GameplayStatics.GetPlayerController` 0) self (`self.StartBlendingTime`) (`self.CameraBlendType`) 0.0 false)
  (bind _asmain_character (cast `/Game/Blueprints/MainCharacter` (`GameplayStatics.GetPlayerCharacter` 0)))
  (set `/Game/Blueprints/MainCharacter.CameraHasChanged` true _asmain_character)
  (`Controller.SetControlRotation` (`GameplayStatics.GetPlayerController` 0) (`SceneComponent.K2_GetComponentRotation` (`self.Camera`))))

(event `DisablePlayerInput`
  ;[1 1 1] Disable Input for the duration of the blend time
  (`self.DisableInput` (`GameplayStatics.GetPlayerCharacter` 0) (`GameplayStatics.GetPlayerController` 0))
  (`KismetSystemLibrary.Delay` (`self.TimedEventAmount`))
  (`self.EnableInput` (`GameplayStatics.GetPlayerCharacter` 0) (`GameplayStatics.GetPlayerController` 0)))

(event `BlendToPlayerCamera`
  ;[1 1 1] Blend back to Player Camera
  (`PlayerController.SetViewTargetWithBlend` (`GameplayStatics.GetPlayerController` 0) (`GameplayStatics.GetPlayerCharacter` 0) (`self.EndBlendingTime`) (`self.CameraBlendType`) 0.0 false)
  (bind _asmain_character (cast `/Game/Blueprints/MainCharacter` (`GameplayStatics.GetPlayerCharacter` 0)))
  (set `/Game/Blueprints/MainCharacter.CameraHasChanged` false _asmain_character))

(event `SingleTimedInstanceEvent`
  ;[1 1 1] Single Timed Instance Event
  (if (`self.SingleTimedInstance`)
    (if (`self.DisablesPlayerInput`)
      (`self.DisablePlayerInput`))
    (`self.BlendToCamera`)
    (`KismetSystemLibrary.Delay` (`self.StartBlendingTime`))
    (`KismetSystemLibrary.Delay` (`self.TimedEventAmount`))
    (`self.BlendToPlayerCamera`)
    (`KismetSystemLibrary.Delay` (`self.EndBlendingTime`))
    (`self.K2_DestroyActor`)))

(event `self.ReceiveBeginPlay`)

(event `AnimateWidgetText`
  ;[1 1 1] Casts to UI_Textbox to animate the Widget Text
  (bind _asui_text_box (cast `/Game/UI/UI_TextBox` (`WidgetComponent.GetUserWidgetObject` (`self.Widget`))))
  (`/Game/UI/UI_TextBox.CreateAnimation` _asui_text_box (`self.WidgetText`)))

(fn `UserConstructionScript`)