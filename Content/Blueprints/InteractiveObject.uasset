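; Puzzle interactable that toggles on or off, swapping material, optionally easing between locations or moving back and forth via timelines, and playing a level sequence or camera event.
; It can toggle linked InteractiveObjects until completed.
; CompletePuzzle checks its required pieces, activates and locks when satisfied, then rechecks every InteractiveObject in the level, so puzzles chain.
; Player overlap swaps highlight mesh and secondary character visibility, shows a widget and sets safe-zone state.
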(event `self.ReceiveBeginPlay`
  ;[1 1 1] Constructor
  (set `self.SpawnLocation` (`self.K2_GetActorLocation`))
  (set `self.RequiredObjects` (`KismetArrayLibrary.Array_Length` (`self.FinalPuzzlePieces`)))
  (bind _returnvalue (`MaterialInterface.GetBaseMaterial` (`PrimitiveComponent.GetMaterial` (`self.StaticMesh`) 0)))
  (set `self.DefaultMaterial` _returnvalue)
  (`self.ParticleEffect`
    (:`then`)
    (:`else`)))

(event `ToggleActivationOfConnected`
  ;[1 1 1] Toggle Activation of this object and all it's connected objects
  (if (not (`self.Completed`))
    (for _array_element (`self.ActivatesTheseInteractiveObjects`)
      (`/Engine/EditorBlueprintResources/StandardMacros.IsValid` _array_element
        (:`Is Valid`
          (`self.ToggleActivation` _array_element))))))

(event `ToggleActivation`
  ;[1 1 1] Toggle Activation of this object and all it's connected objects
  (if (not (`self.Completed`))
    (`KismetSystemLibrary.Delay` (`self.DelayActivation`))
    (set `self.Activated` (not (`self.Activated`)))
    (`self.ToggleActivateAnimation`)
    (`self.PlayCinematic`)
    (if (`self.Movable`)
      (if (`self.ConstantBackAndForward`)
        (`self.ActivateBackAndForth`)
        (else
          (`self.ActivateToggleLocation` (`self.Activated`)))))))

(event `self.Sphere.OnComponentBeginOverlap`
  (params (OverlappedComponent :type "PrimitiveComponent Object Reference") (OtherActor :type "Actor Object Reference") (OtherComp :type "PrimitiveComponent Object Reference") (OtherBodyIndex :type Integer) (bFromSweep :type Boolean) (SweepResult :type "HitResult Structure (by ref)"))
  ;[1 1 1] Toggle Highlighting when Main Character is close by
  (if (== OtherActor (`GameplayStatics.GetPlayerCharacter` 0))
    (set `self.Inside` true)
    (if (`self.Clickable`)
      (`SceneComponent.SetVisibility` (`self.SkeletalMesh`) true false)
      (bind _asmain_character (cast `/Game/Blueprints/MainCharacter` OtherActor))
      (`SceneComponent.SetVisibility` (`/Game/Blueprints/MainCharacter.SecondaryCharacter` _asmain_character) false false)
      (if (`self.ShowWidget`)
        (`SceneComponent.SetVisibility` (`self.Widget`) true false)
        (if (`self.SafeZone`)
          (bind _asmain_character_2 (cast `/Game/Blueprints/MainCharacter` (`GameplayStatics.GetPlayerCharacter` 0)))
          (set `/Game/Blueprints/MainCharacter.InSafeZone` true _asmain_character_2))))))

(event `self.Sphere.OnComponentEndOverlap`
  (params (OverlappedComponent :type "PrimitiveComponent Object Reference") (OtherActor :type "Actor Object Reference") (OtherComp :type "PrimitiveComponent Object Reference") (OtherBodyIndex :type Integer))
  ;[1 1 1] Toggle Highlighting when Main Character is close by
  (if (== OtherActor (`GameplayStatics.GetPlayerCharacter` 0))
    (set `self.Inside` false)
    (`SceneComponent.SetVisibility` (`self.SkeletalMesh`) false false)
    (bind _asmain_character (cast `/Game/Blueprints/MainCharacter` OtherActor))
    (`SceneComponent.SetVisibility` (`/Game/Blueprints/MainCharacter.SecondaryCharacter` _asmain_character) true false)
    (if (`self.ShowWidget`)
      (`SceneComponent.SetVisibility` (`self.Widget`) false false)
      (if (`self.SafeZone`)
        (bind _asmain_character_2 (cast `/Game/Blueprints/MainCharacter` (`GameplayStatics.GetPlayerCharacter` 0)))
        (set `/Game/Blueprints/MainCharacter.InSafeZone` false _asmain_character_2)))))

(event `ActivateToggleLocation`
  (params (ToggledActivation :type Boolean))
  ;[1 1 1] Toggle Location using a Timeline via Ease function
  (if ToggledActivation
    (`TimelineComponent.SetPlayRate` (`self.Timeline_Move`) (/ 1.0 (`self.PlayRateSpeedInSeconds`)))
    (bind (_direction _track) (`Timeline|Timeline_Move` :!label _label)
      (:`Update`
        (`self.K2_SetActorLocation` (`|EaseFunction` (`self.MovingType`) _track (`self.SpawnLocation`) (+ (`self.SpawnLocation`) (`self.EndLocationPosition`)) 1.0))))
    (else
      (goto _label :!via `Reverse`))))

(event `ToggleActivateAnimation`
  ;[1 1 1] ToggleActivateAnimation
  (if (`self.Activated`)
    (bind _activatedmaterial (`self.ActivatedMaterial`)
      (:`then`
        (`PrimitiveComponent.SetMaterial` (`self.StaticMesh`) 0 _activatedmaterial))
      (:`else`))
    (else
      (`PrimitiveComponent.SetMaterial` (`self.StaticMesh`) 0 (`self.DefaultMaterial`)))))

(event `CompletePuzzle`
  ;[1 1 1] Checks Completion of this puzzle
  (if (> (`KismetArrayLibrary.Array_Length` (`self.FinalPuzzlePieces`)) 0)
    (set `self.ActivatedObjects` 0)
    (for _array_element (`self.FinalPuzzlePieces`)
      (`/Engine/EditorBlueprintResources/StandardMacros.IsValid` _array_element
        (:`Is Valid`
          (if (`/Game/Blueprints/InteractiveObject.Activated` _array_element)
            (`/Engine/EditorBlueprintResources/StandardMacros.IncrementInt` (`self.ActivatedObjects`))
            (else
              (set `self.ActivatedObjects` 0))))))
    (if (and (== (`self.RequiredObjects`) (`self.ActivatedObjects`)) (> (+ (`self.RequiredObjects`) (`self.ActivatedObjects`)) 0))
      (`self.ToggleActivation`)
      (set `self.Completed` true)
      (for _array_element_2 (`self.FinalPuzzlePieces`)
        (set `/Game/Blueprints/InteractiveObject.Completed` true _array_element_2)
        (`KismetSystemLibrary.Delay` 0.1)
        (`self.CheckAllPuzzlesForCompletion`)))))

(event `CheckAllPuzzlesForCompletion`
  ;[1 1 1] Checks Completion of this puzzle
  ;;[1 1 1] Checks all Interactible Objects in the Level for completion
  (bind _outactors (`GameplayStatics.GetAllActorsOfClass` "InteractiveObject_C"))
  (for _array_element _outactors
    (`self.CompletePuzzle` _array_element)))

(event `PlayCinematic`
  ;[1 1 1] Play Level Sequence
  (`self.LevelSequence`
    (:`then`
      (bind (_outactor _returnvalue) (`LevelSequencePlayer.CreateLevelSequencePlayer` (`self.LevelSequence`)))
      (bind _outactors (`GameplayStatics.GetAllActorsOfClass` "/Game/Blueprints/KeyOfLifeGameMode.KeyOfLifeGameMode_C"))
      (for _array_element _outactors
        (`/Game/Blueprints/KeyOfLifeGameMode.PlayLevelSequence` _array_element _returnvalue)))
    (:`else`
      (bind _cameraarea (`self.CameraArea`)
        (:`then`
          (`/Game/Blueprints/CameraArea.SingleTimedInstanceEvent` _cameraarea))
        (:`else`)))))

(event `ActivateBackAndForth`
  ;[1 1 1] Toggle Back And Forth
  (if (`self.Activated`)
    (`TimelineComponent.SetPlayRate` (`self.Timeline_BackAndForth`) (/ 1.0 (`self.PlayRateSpeedInSeconds`)))
    (bind (_direction _track) (`Timeline|Timeline_BackAndForth`)
      (:`Update`
        (`self.K2_SetActorLocation` (`|EaseFunction` (`self.MovingType`) _track (`self.SpawnLocation`) (+ (`self.SpawnLocation`) (`self.EndLocationPosition`)) 1.0))))
    (else
      (`TimelineComponent.Stop` (`self.Timeline_BackAndForth`)))))

(fn `UserConstructionScript`)