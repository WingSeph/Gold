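; Recurring shockwave hazard that respawns a player caught inside its sphere outside a safe zone.
; A self-re-triggering delay loop runs the overlap check, then the blast shortly after, then waits DangerSeconds.
; Each blast spawns a new RadialForceActor sized to the sphere, firing its impulse only if the player is outside a safe zone.
; Sound, camera shake and particles play on every blast regardless.
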(event `self.ReceiveBeginPlay`
  (`self.ShockwaveEvent`)
  (set `self.ShockwaveRadius` (`SphereComponent.GetScaledSphereRadius` (`self.SphereCollision`))))

(event `ShockwaveEvent`
  (`KismetSystemLibrary.Delay` 0.2)
  (`self.CheckPlayerOverlapping`)
  (`KismetSystemLibrary.Delay` 0.1)
  (`self.ShockwaveBlast`)
  (`KismetSystemLibrary.Delay` (`self.DangerSeconds`))
  (`self.ShockwaveEvent`))

(event `ShockwaveBlast`
  (bind _returnvalue (`|SpawnActorFromClass` "/Script/Engine.RadialForceActor" (`self.GetTransform`) "Undefined" "OverrideRootScale" null null))
  (bind _forcecomponent (`RadialForceActor.ForceComponent` _returnvalue))
  (set `RadialForceComponent.Radius` (`self.ShockwaveRadius`) _forcecomponent)
  (set `RadialForceComponent.ImpulseStrength` 500000.0 _forcecomponent)
  (bind _asmain_character (cast `/Game/Blueprints/MainCharacter` (`GameplayStatics.GetPlayerCharacter` 0)))
  (if (not (`/Game/Blueprints/MainCharacter.InSafeZone` _asmain_character))
    (`RadialForceComponent.FireImpulse` _forcecomponent))
  (`GameplayStatics.PlaySoundAtLocation` "/Game/StarterContent/Audio/Explosion_Cue.Explosion_Cue" (`self.K2_GetActorLocation`) (struct) 1.0 1.0 0.0 null null null)
  (`GameplayStatics.PlayWorldCameraShake` "/Game/Art/Sound/Sounds/platform_shake.platform_shake_C" (`self.K2_GetActorLocation`) 0.0 (`self.ShockwaveRadius`))
  (`GameplayStatics.SpawnEmitterAtLocation` "/Game/J_VFX/Shockwave_VFX/p_bigboi_shock.p_bigboi_shock" (`self.K2_GetActorLocation`) (struct) (* (`self.GetActorScale3D`) 0.2)))

(event `CheckPlayerOverlapping`
  ;[1 1 1] Check if player is inside the sphere collision box
  (if (`PrimitiveComponent.IsOverlappingActor` (`self.SphereCollision`) (`GameplayStatics.GetPlayerCharacter` 0))
    (bind _asmain_character (cast `/Game/Blueprints/MainCharacter` (`GameplayStatics.GetPlayerCharacter` 0)))
    (if (not (`/Game/Blueprints/MainCharacter.InSafeZone` _asmain_character))
      (`/Game/Blueprints/MainCharacter.Respawn` _asmain_character))))

(fn `UserConstructionScript`)