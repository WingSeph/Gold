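; TransitionToLevel is a trigger volume Blueprint that moves the player to another level.
; When a MainCharacter overlaps its Box, it starts a camera fade and disables the player character's input.
; After a delay matching the fade duration, it opens the level named by the LevelToLoad variable.
; The end-overlap event only casts and has no further effect.
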(event `self.Box.OnComponentBeginOverlap`
  (params (OverlappedComponent :type "PrimitiveComponent Object Reference") (OtherActor :type "Actor Object Reference") (OtherComp :type "PrimitiveComponent Object Reference") (OtherBodyIndex :type Integer) (bFromSweep :type Boolean) (SweepResult :type "HitResult Structure (by ref)"))
  (cast `/Game/Blueprints/MainCharacter` OtherActor)
  (`PlayerCameraManager.StartCameraFade` :`self` (`GameplayStatics.GetPlayerCameraManager` 0) :`FromAlpha` 0.2 :`ToAlpha` 3.0 :`Duration` 5.0)
  (`self.DisableInput` (`GameplayStatics.GetPlayerCharacter` 0) (`GameplayStatics.GetPlayerController` 0))
  (`KismetSystemLibrary.Delay` 5.0)
  (`GameplayStatics.OpenLevel` (`self.LevelToLoad`)))

(event `self.Box.OnComponentEndOverlap`
  (params (OverlappedComponent :type "PrimitiveComponent Object Reference") (OtherActor :type "Actor Object Reference") (OtherComp :type "PrimitiveComponent Object Reference") (OtherBodyIndex :type Integer))
  (cast `/Game/Blueprints/MainCharacter` OtherActor))

(fn `UserConstructionScript`)