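; BP_DoorDissolve is a door that dissolves as the player character enters its box trigger and reverses when they leave.
; BeginPlay creates dynamic material instances for three DoorLuke material slots, one dissolve texture and two gold dissolve.
; Overlap events play or reverse a dissolve timeline, whose track is meant to drive the dissolveAmount scalar on all three instances.
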(event `self.ReceiveBeginPlay`
  (`|ExecutionSequence`
    (:`then_0`
      (bind _returnvalue (`PrimitiveComponent.CreateDynamicMaterialInstance` (`self.Door_luke`) 0 "/Game/Art/VFX/DoorDisintegrate/M_DissolveTexture_Inst.M_DissolveTexture_Inst" "None")))
    (:`then_1`
      (bind _returnvalue_2 (`PrimitiveComponent.CreateDynamicMaterialInstance` (`self.Door_luke`) 1 "/Game/Art/VFX/DoorDisintegrate/M_DissolveGold.M_DissolveGold" "None")))
    (:`then_2`
      (bind _returnvalue_3 (`PrimitiveComponent.CreateDynamicMaterialInstance` (`self.Door_luke`) 2 "/Game/Art/VFX/DoorDisintegrate/M_DissolveGold.M_DissolveGold" "None")))))

(event `self.BoxCollision.OnComponentBeginOverlap`
  (params (OverlappedComponent :type "PrimitiveComponent Object Reference") (OtherActor :type "Actor Object Reference") (OtherComp :type "PrimitiveComponent Object Reference") (OtherBodyIndex :type Integer) (bFromSweep :type Boolean) (SweepResult :type "HitResult Structure (by ref)"))
  (if (== OtherActor (`GameplayStatics.GetPlayerCharacter` 0))
    (`TimelineComponent.Play` (`self.Timeline_Dissolve`))))

(event `self.BoxCollision.OnComponentEndOverlap`
  (params (OverlappedComponent :type "PrimitiveComponent Object Reference") (OtherActor :type "Actor Object Reference") (OtherComp :type "PrimitiveComponent Object Reference") (OtherBodyIndex :type Integer))
  (if (== OtherActor (`GameplayStatics.GetPlayerCharacter` 0))
    (`TimelineComponent.Reverse` (`self.Timeline_Dissolve`))))

(fn `UserConstructionScript`)