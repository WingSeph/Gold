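; Puzzle pressure platform that toggles linked InteractiveObjects when stepped on, with particle, material, sound and camera shake feedback.
; Box overlaps ignore NPC and InteractiveObject triggers but count characters, pickups and interactive objects to detect first entry and last exit.
; Activation prompts each linked object to check puzzle completion after a short delay.
; Leaving deactivates it unless single-activation or timed; a Tick countdown deactivates timed, reusable platforms.
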(event `self.ReceiveBeginPlay`
  ;[1 1 1] Begin Play
  (set `self.Timer` (`self.MaxTimer`)))

(event `self.Box.OnComponentBeginOverlap`
  (params (OverlappedComponent :type "PrimitiveComponent Object Reference") (OtherActor :type "Actor Object Reference") (OtherComp :type "PrimitiveComponent Object Reference") (OtherBodyIndex :type Integer) (bFromSweep :type Boolean) (SweepResult :type "HitResult Structure (by ref)"))
  ;[1 1 1] Overlap
  (cast `/Game/Blueprints/NPC_Class` OtherActor
    (:`CastFailed`
      (cast `/Game/Blueprints/InteractiveObject` OtherActor
        (:`CastFailed`
          (if true
            (if (<= (+ (`KismetArrayLibrary.Array_Length` (`PrimitiveComponent.GetOverlappingActors` (`self.Box`) "/Game/Blueprints/MainCharacter.MainCharacter_C")) (`KismetArrayLibrary.Array_Length` (`PrimitiveComponent.GetOverlappingActors` (`self.Box`) "/Game/Blueprints/PickUpMaker.PickUpMaker_C")) (`KismetArrayLibrary.Array_Length` (`PrimitiveComponent.GetOverlappingActors` (`self.Box`) "/Game/Blueprints/InteractiveObject.InteractiveObject_C"))) 1)
              (if (not (`self.Activated`))
                (`self.ActivateAllQuestComponents`)
                (`KismetSystemLibrary.Delay` 0.1)
                (for _array_element (`self.InteractiveObjects`)
                  (`/Game/Blueprints/InteractiveObject.CheckAllPuzzlesForCompletion` _array_element))))))))))

(event `self.Box.OnComponentEndOverlap`
  (params (OverlappedComponent :type "PrimitiveComponent Object Reference") (OtherActor :type "Actor Object Reference") (OtherComp :type "PrimitiveComponent Object Reference") (OtherBodyIndex :type Integer))
  ;[1 1 1] Overlap
  (cast `/Game/Blueprints/NPC_Class` OtherActor
    (:`CastFailed`
      (cast `/Game/Blueprints/InteractiveObject` OtherActor
        (:`CastFailed`
          (if true
            (if (<= (+ (`KismetArrayLibrary.Array_Length` (`PrimitiveComponent.GetOverlappingActors` (`self.Box`) "/Game/Blueprints/MainCharacter.MainCharacter_C")) (`KismetArrayLibrary.Array_Length` (`PrimitiveComponent.GetOverlappingActors` (`self.Box`) "/Game/Blueprints/PickUpMaker.PickUpMaker_C")) (`KismetArrayLibrary.Array_Length` (`PrimitiveComponent.GetOverlappingActors` (`self.Box`) "/Game/Blueprints/InteractiveObject.InteractiveObject_C"))) 0)
              (if (not (or (`self.SingleActivationOnly`) (`self.Timed`)))
                (`self.DeactivateAllQuestComponents`)))))))))

(event `ActiveAnimation`
  ;[1 1 1] Animation
  (`SceneComponent.SetVisibility` (`self.ParticleSystem`) true false)
  (`PrimitiveComponent.SetMaterial` (`self.Platform`) 2 (`self.Material_Highlighted`))
  (`GameplayStatics.PlaySoundAtLocation` "/Game/Art/Sound/tech/swoosh_meta_L_R_006_Cue.swoosh_meta_L_R_006_Cue" (`self.K2_GetActorLocation` self) (struct) 0.15 1.0 0.0 null null null)
  (`GameplayStatics.PlayWorldCameraShake` "/Game/Art/Sound/Sounds/platform_shake.platform_shake_C" (`self.K2_GetActorLocation` self) 0.0 10000.0))

(event `InactiveAnimation`
  ;[1 1 1] Animation
  (`SceneComponent.SetVisibility` (`self.ParticleSystem`) false false)
  (`PrimitiveComponent.SetMaterial` (`self.Platform`) 2 (`self.Material_Normal`))
  (`GameplayStatics.PlaySoundAtLocation` "/Game/Art/Sound/tech/swoosh_meta_L_R_006_Cue.swoosh_meta_L_R_006_Cue" (`self.K2_GetActorLocation` self) (struct) 0.15 0.6 0.0 null null null)
  (`GameplayStatics.PlayWorldCameraShake` "/Game/Art/Sound/Sounds/platform_shake.platform_shake_C" (`self.K2_GetActorLocation` self) 0.0 10000.0))

(event `ActivateAllQuestComponents`
  ;[1 1 1] Activate and Deactivate
  (for _array_element (`self.InteractiveObjects`)
    (`/Game/Blueprints/InteractiveObject.ToggleActivation` _array_element))
  (set `self.Activated` true)
  (`self.ActiveAnimation`))

(event `DeactivateAllQuestComponents`
  ;[1 1 1] Activate and Deactivate
  (for _array_element (`self.InteractiveObjects`)
    (`/Game/Blueprints/InteractiveObject.ToggleActivation` _array_element))
  (set `self.Activated` false)
  (`self.InactiveAnimation`))

(event `TimerEvent`
  ;[1 1 1] Timer Event
  (if (`self.Timed`)
    (if (`self.SingleActivationOnly`)
      _
      (elif (`self.Activated`)
        (set `self.Timer` (- (`self.Timer`) (`GameplayStatics.GetWorldDeltaSeconds`)))
        (if (<= (`self.Timer`) 0.0)
          (`self.DeactivateAllQuestComponents`)
          (set `self.Timer` (`self.MaxTimer`)))))))

(event `self.ReceiveTick`
  (params (DeltaSeconds :type "Float (single-precision)"))
  ;[1 1 1] Timer Event
  (`self.TimerEvent`))

(fn `UserConstructionScript`)