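; Pickup object actor that reacts to a nearby MainCharacter and can lock onto a Quest_Platform.
; Its Sphere overlap sets PlayerInRange and swaps visibility, showing its own SkeletalMesh and hiding the character's SecondaryCharacter, then reversing on exit.
; LockIntoPlatform, called on BeginPlay, teleports the Cube to any overlapping Quest_Platform and turns off its physics simulation.
; The graph contains no grab or carry logic.
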(event `self.ReceiveBeginPlay`
  (`self.LockIntoPlatform`))

(event `self.Sphere.OnComponentBeginOverlap`
  (params (OverlappedComponent :type "PrimitiveComponent Object Reference") (OtherActor :type "Actor Object Reference") (OtherComp :type "PrimitiveComponent Object Reference") (OtherBodyIndex :type Integer) (bFromSweep :type Boolean) (SweepResult :type "HitResult Structure (by ref)"))
  ;[1 1 1] Overlap
  (bind _asmain_character (cast `/Game/Blueprints/MainCharacter` OtherActor))
  (`SceneComponent.SetVisibility` (`/Game/Blueprints/MainCharacter.SecondaryCharacter` _asmain_character) false false)
  (`SceneComponent.SetVisibility` (`self.SkeletalMesh`) true false)
  (set `self.PlayerInRange` true))

(event `self.Sphere.OnComponentEndOverlap`
  (params (OverlappedComponent :type "PrimitiveComponent Object Reference") (OtherActor :type "Actor Object Reference") (OtherComp :type "PrimitiveComponent Object Reference") (OtherBodyIndex :type Integer))
  ;[1 1 1] Overlap
  (bind _asmain_character (cast `/Game/Blueprints/MainCharacter` OtherActor))
  (`SceneComponent.SetVisibility` (`/Game/Blueprints/MainCharacter.SecondaryCharacter` _asmain_character) true false)
  (`SceneComponent.SetVisibility` (`self.SkeletalMesh`) false false)
  (set `self.PlayerInRange` false))

(event `LockIntoPlatform`
  (for _array_element (`self.GetOverlappingActors` "/Game/Blueprints/Quest_Platform.Quest_Platform_C")
    (`SceneComponent.K2_SetWorldLocation` (`self.Cube`) (+ (`SceneComponent.K2_GetComponentLocation` (`Actor.RootComponent` _array_element)) (0.0 0.0 0.0)) true true)
    (`PrimitiveComponent.SetSimulatePhysics` (`self.Cube`) false)))

(fn `UserConstructionScript`)