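; RespawnPoint is a checkpoint actor that sets where the MainCharacter respawns.
; When the MainCharacter overlaps its Sphere, it writes its own location to the character's RespawnLocation.
; A point flagged StartingSpawn also writes its location to the player character on BeginPlay, providing the initial respawn location.
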(event `self.ReceiveBeginPlay`
  (if (`self.StartingSpawn?`)
    (bind _asmain_character (cast `/Game/Blueprints/MainCharacter` (`GameplayStatics.GetPlayerCharacter` 0)))
    (set `/Game/Blueprints/MainCharacter.RespawnLocation` (`self.K2_GetActorLocation` self) _asmain_character)))

(event `self.Sphere.OnComponentBeginOverlap`
  (params (OverlappedComponent :type "PrimitiveComponent Object Reference") (OtherActor :type "Actor Object Reference") (OtherComp :type "PrimitiveComponent Object Reference") (OtherBodyIndex :type Integer) (bFromSweep :type Boolean) (SweepResult :type "HitResult Structure (by ref)"))
  (bind _asmain_character (cast `/Game/Blueprints/MainCharacter` OtherActor))
  (set `/Game/Blueprints/MainCharacter.RespawnLocation` (`self.K2_GetActorLocation` self) _asmain_character))

(fn `UserConstructionScript`)