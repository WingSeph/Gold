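; Game mode for KeyOfLife that plays level sequences with an on-screen tab-to-skip prompt.
; PlayLevelSequence stores and plays the given sequence player, shows a UI_TabToSkip widget, then removes it after a delay equal to the sequence's duration.
; StopLevelSequence halts a valid player and removes the prompt early.
; BeginPlay also seeds a freshly made random stream.
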(event `self.ReceiveBeginPlay`
  (`KismetMathLibrary.SeedRandomStream` (`KismetMathLibrary.MakeRandomStream` (`KismetMathLibrary.RandomInteger` 0))))

(event `StopLevelSequence`
  (`/Engine/EditorBlueprintResources/StandardMacros.IsValid` (`self.SequencePlayer`)
    (:`Is Valid`
      (`MovieSceneSequencePlayer.Stop` (`self.SequencePlayer`))
      (`Widget.RemoveFromParent` (stale `PlayLevelSequence` _returnvalue)))))

(event `PlayLevelSequence`
  (params (NewSequence :type "LevelSequencePlayer Object Reference"))
  (bind _sequenceplayer (`self.SequencePlayer`))
  (set `self.SequencePlayer` NewSequence)
  (`MovieSceneSequencePlayer.Play` _sequenceplayer)
  (bind _returnvalue (`|CreateWidget` "/Game/UI/UI_TabToSkip.UI_TabToSkip_C" (`GameplayStatics.GetPlayerController` 0)))
  (`UserWidget.AddToViewport` _returnvalue 0)
  (`KismetSystemLibrary.Delay` (`TimeManagementBlueprintLibrary.Conv_QualifiedFrameTimeToSeconds` (`MovieSceneSequencePlayer.GetDuration` _sequenceplayer)))
  (`Widget.RemoveFromParent` _returnvalue))

(fn `UserConstructionScript`)