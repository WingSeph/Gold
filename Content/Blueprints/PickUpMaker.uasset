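; Pickup sphere actor that the player can carry, drop and place on a Quest_Platform.
; Tick-polled state flags teleport the held sphere to MainCharacter's SecondaryCharacter, or snap a dropped, physics-simulated sphere above an overlapping platform.
; PickUpSphere and DropSphere toggle physics and highlight material, with a pulse emitter on highlight; DropSphere leaves Held set.
; Pedestal overlaps call a levitation timeline behind Held checks; its update and the dissolve logic are unwired.
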(event `self.ReceiveBeginPlay`
  ;[1 1 1] Begin Play
  (set `self.DefaultSphereLocation` (`SceneComponent.K2_GetComponentLocation` (`self.Sphere`))))

(event `self.ReceiveTick`
  (params (DeltaSeconds :type "Float (single-precision)"))
  ;[1 1 1] Tick
  (`self.HeldEvent`)
  (`self.PlatformEvent`)
  (`self.DroppedEvent`))

(event `self.Collision.OnComponentBeginOverlap`
  (params (OverlappedComponent :type "PrimitiveComponent Object Reference") (OtherActor :type "Actor Object Reference") (OtherComp :type "PrimitiveComponent Object Reference") (OtherBodyIndex :type Integer) (bFromSweep :type Boolean) (SweepResult :type "HitResult Structure (by ref)"))
  ;[1 1 1] Overlapping Events
  (if (== OtherActor (`GameplayStatics.GetPlayerCharacter` 0))
    (set `self.Overlapping` true)))

(event `self.Collision.OnComponentEndOverlap`
  (params (OverlappedComponent :type "PrimitiveComponent Object Reference") (OtherActor :type "Actor Object Reference") (OtherComp :type "PrimitiveComponent Object Reference") (OtherBodyIndex :type Integer))
  ;[1 1 1] Overlapping Events
  (if (== OtherActor (`GameplayStatics.GetPlayerCharacter` 0))
    (set `self.Overlapping` false)))

(event `self.Collision_Pedestal.OnComponentBeginOverlap`
  (params (OverlappedComponent :type "PrimitiveComponent Object Reference") (OtherActor :type "Actor Object Reference") (OtherComp :type "PrimitiveComponent Object Reference") (OtherBodyIndex :type Integer) (bFromSweep :type Boolean) (SweepResult :type "HitResult Structure (by ref)"))
  ;[1 1 1] Overlapping Events
  (if (== OtherActor (`GameplayStatics.GetPlayerCharacter` 0))
    (set `self.Overlapping` true)
    (if (`self.OnPlatform`)
      _
      (elif (`self.Dropped`)
        _
        (elif (`self.Held`)
          (`self.Animate_Activate`))))))

(event `self.Collision_Pedestal.OnComponentEndOverlap`
  (params (OverlappedComponent :type "PrimitiveComponent Object Reference") (OtherActor :type "Actor Object Reference") (OtherComp :type "PrimitiveComponent Object Reference") (OtherBodyIndex :type Integer))
  ;[1 1 1] Overlapping Events
  (if (== OtherActor (`GameplayStatics.GetPlayerCharacter` 0))
    (set `self.Overlapping` false)
    (if (`self.OnPlatform`)
      _
      (elif (`self.Dropped`)
        _
        (elif (not (`self.Held`))
          (`self.Animate_Deactivate`))))))

(event `Animate_Activate`
  ;[1 1 1] Animation Events
  (if (not (`self.Held`))
    (`TimelineComponent.SetLooping` (`self.Timeline_AnimateSphere`) true)
    (`TimelineComponent.Play` (`self.Timeline_AnimateSphere`))))

(event `Animate_Deactivate`
  ;[1 1 1] Animation Events
  (if (not (`self.Held`))
    (`TimelineComponent.SetLooping` (`self.Timeline_AnimateSphere`) false)
    (`TimelineComponent.Reverse` (`self.Timeline_AnimateSphere`))))

(event `Animate_Highlight`
  ;[1 1 1] Animation Events
  (set `self.Highlighted` true)
  (`PrimitiveComponent.SetMaterial` (`self.Sphere`) 0 (`self.Material_Highlighted`))
  (`GameplayStatics.SpawnEmitterAtLocation` "/Game/Art/Materials/scan/P_Pulse.P_Pulse" (`SceneComponent.K2_GetComponentLocation` (`self.Sphere`)))
  (`KismetSystemLibrary.Delay` 3.0)
  (if (`self.Held`)
    _
    (elif (`self.Overlapping`)
      _
      (elif (not (`self.OnPlatform`))
        (`self.Animate_DeHighlight`)))))

(event `Animate_DeHighlight`
  ;[1 1 1] Animation Events
  (set `self.Highlighted` false)
  (`PrimitiveComponent.SetMaterial` (`self.Sphere`) 0 (`self.Material_Normal`)))

(event `HeldEvent`
  ;[1 1 1] Tick Events
  (if (`self.Held`)
    (bind _asmain_character (cast `/Game/Blueprints/MainCharacter` (`GameplayStatics.GetPlayerCharacter` 0)))
    (`SceneComponent.K2_SetWorldLocation` (`self.Sphere`) (`SceneComponent.K2_GetComponentLocation` (`/Game/Blueprints/MainCharacter.SecondaryCharacter` _asmain_character)) false true)))

(event `PlatformEvent`
  ;[1 1 1] Tick Events
  (if (`self.OnPlatform`)
    (bind _questplatform (`self.QuestPlatform`)
      (:`then`
        (`SceneComponent.K2_SetWorldLocation` (`self.Sphere`) (+ (`self.K2_GetActorLocation` _questplatform) (* (`self.GetActorUpVector` _questplatform) 100.0)) false true))
      (:`else`))))

(event `DroppedEvent`
  ;[1 1 1] Tick Events
  (if (`self.Dropped`)
    (`self.CheckForPlatform`)))

(event `CheckForPlatform`
  (bind _overlappingactors (`PrimitiveComponent.GetOverlappingActors` (`self.Collision`) "/Game/Blueprints/Quest_Platform.Quest_Platform_C"))
  ;[1 1 1] Tick Events
  (if (> (`KismetArrayLibrary.Array_Length` _overlappingactors) 0)
    (for _array_element _overlappingactors
      (set `self.QuestPlatform` _array_element)
      (set `self.Dropped` false)
      (set `self.OnPlatform` true)
      (`PrimitiveComponent.SetSimulatePhysics` (`self.Sphere`) false)
      (`PrimitiveComponent.SetCollisionEnabled` (`self.Sphere`) "NoCollision")
      (`self.Animate_Highlight`))))

(event `ReturnSphereToDefaultLocation`
  ;[1 1 1] Return Sphere to Default Location
  (`SceneComponent.K2_SetWorldLocation` (`self.Sphere`) (`self.DefaultSphereLocation`) false true))

(event `DropSphere`
  ;[1 1 1] Drop Events
  (set `self.Dropped` true)
  (`PrimitiveComponent.SetCollisionEnabled` (`self.Sphere`) "QueryAndPhysics")
  (`PrimitiveComponent.SetSimulatePhysics` (`self.Sphere`) true)
  (`self.Animate_DeHighlight`))

(event `PickUpSphere`
  ;[1 1 1] Drop Events
  (set `self.Dropped` false)
  (set `self.OnPlatform` false)
  (set `self.Held` true)
  (`PrimitiveComponent.SetSimulatePhysics` (`self.Sphere`) false)
  (`PrimitiveComponent.SetCollisionEnabled` (`self.Sphere`) "NoCollision")
  (`TimelineComponent.Stop` (`self.Timeline_AnimateSphere`))
  (`self.Animate_Highlight`))

(fn `UserConstructionScript`)