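; BP_Sphere is a helper actor in the MeshDissolve material folder that feeds its Cube component's transform to the PC_Data material parameter collection.
; The construction script writes the world location to "Position 1" and the X world scale to "Radius".
; BeginPlay rewrites "Position 1" but writes the full scale vector to "Bounds" instead of updating "Radius".
; Tick is disabled, so movement during play is not tracked here.
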(event `self.ReceiveBeginPlay`
  (bind _cube (`self.Cube`))
  (`KismetMaterialLibrary.SetVectorParameterValue` "/Game/Art/Materials/MeshDissolve/PC_Data.PC_Data" "Position 1" (`KismetMathLibrary.Conv_VectorToLinearColor` (`SceneComponent.K2_GetComponentLocation` _cube)))
  (`KismetMaterialLibrary.SetVectorParameterValue` "/Game/Art/Materials/MeshDissolve/PC_Data.PC_Data" "Bounds" (`KismetMathLibrary.Conv_VectorToLinearColor` (`SceneComponent.K2_GetComponentScale` _cube))))

(fn `UserConstructionScript`
  (bind _cube (`self.Cube`))
  (bind _returnvalue_x (`KismetMathLibrary.BreakVector` (`SceneComponent.K2_GetComponentScale` _cube)))
  (`KismetMaterialLibrary.SetVectorParameterValue` "/Game/Art/Materials/MeshDissolve/PC_Data.PC_Data" "Position 1" (`KismetMathLibrary.Conv_VectorToLinearColor` (`SceneComponent.K2_GetComponentLocation` _cube)))
  (`KismetMaterialLibrary.SetScalarParameterValue` "/Game/Art/Materials/MeshDissolve/PC_Data.PC_Data" "Radius" _returnvalue_x))