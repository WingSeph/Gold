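; BP_Cube is a mesh dissolve helper that publishes its cube's placement to materials.
; It writes the Cube component's world location and world scale into the PC_Data material parameter collection as "Position 1" and "Bounds 1".
; The write runs in the construction script and again at BeginPlay, with no per-tick update.
; The parameter names are fixed, so every instance writes to the same slot.
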(event `self.ReceiveBeginPlay`
  (bind _cube (`self.Cube`))
  (`KismetMaterialLibrary.SetVectorParameterValue` "/Game/Art/Materials/MeshDissolve/PC_Data.PC_Data" "Position 1" (`KismetMathLibrary.Conv_VectorToLinearColor` (`SceneComponent.K2_GetComponentLocation` _cube)))
  (`KismetMaterialLibrary.SetVectorParameterValue` "/Game/Art/Materials/MeshDissolve/PC_Data.PC_Data" "Bounds 1" (`KismetMathLibrary.Conv_VectorToLinearColor` (`SceneComponent.K2_GetComponentScale` _cube))))

(fn `UserConstructionScript`
  (bind _cube (`self.Cube`))
  (`KismetMaterialLibrary.SetVectorParameterValue` "/Game/Art/Materials/MeshDissolve/PC_Data.PC_Data" "Position 1" (`KismetMathLibrary.Conv_VectorToLinearColor` (`SceneComponent.K2_GetComponentLocation` _cube)))
  (`KismetMaterialLibrary.SetVectorParameterValue` "/Game/Art/Materials/MeshDissolve/PC_Data.PC_Data" "Bounds 1" (`KismetMathLibrary.Conv_VectorToLinearColor` (`SceneComponent.K2_GetComponentScale` _cube))))